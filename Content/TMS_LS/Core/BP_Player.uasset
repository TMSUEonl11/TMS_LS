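; Player Blueprint whose event graph holds only debug hotkeys and disconnected test nodes.
; X adds a stack of red potions through InventoryComponent and randomizes the WaterColor parameter in the MPC_Weather collection.
; Z fires forward object and channel line traces from the actor, drawing only the object trace and ignoring both results.
; Unwired leftovers touch GAS stamina-drain effects and the inventory subsystem; BeginPlay, Tick and overlap events are empty.
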(event EventBeginPlay)

(event Collision|EventActorBeginOverlap
  (params (OtherActor :type Actor%20Object%20Reference)))

(event EventTick
  (params (DeltaSeconds :type Float%20%28single-precision%29)))

(event Input|KeyboardEvents|DebugKeyZ
  (params (Key :type Key%20Structure :default "None") (ActionValue :type Input%20Action%20Value%20Structure))
  (bind _returnvalue (Transformation|GetActorLocation))
  (bind _returnvalue_2 (Transformation|GetActorForwardVector))
  (bind _returnvalue_3 (* _returnvalue_2 1e+03))
  (bind _returnvalue_4 (+ _returnvalue _returnvalue_3))
  (:Pressed
    (Collision|LineTraceForObjects _returnvalue _returnvalue_4 (Utilities|Array|MakeArray "ObjectTypeQuery7") false 0 "ForDuration")
    (Collision|LineTraceByChannel _returnvalue _returnvalue_4 "TraceTypeQuery3" false 0 "None")))

(event Input|KeyboardEvents|DebugKeyX
  (params (Key :type Key%20Structure :default "None") (ActionValue :type Input%20Action%20Value%20Structure))
  (:Pressed
    (Class|TMSInventoryComponent|AddItem (Variables|Default|GetInventoryComponent) (Utilities|Struct|MakeItemSlotData "RedPotion" 37))
    (Rendering|Material|SetVectorParameterValue "/Game/TMS_LS/Materials/PostProcess/MPC_Weather.MPC_Weather" "WaterColor" (Math|Conversions|ToLinearColor(Vector) (Math|Random|RandomUnitVector)) :!class /Script/Engine.KismetMaterialLibrary)))

(fn ConstructionScript)