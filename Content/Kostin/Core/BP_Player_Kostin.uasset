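; BP_Player_Kostin is a player Blueprint that binds debug keys for testing item data lookup and world interaction.
; T prints the name of item 0 from GameInstanceSubsystemKostin.
; E sphere-traces from the actor's location along the camera's forward vector and sends InteractCallMessage with the player controller to hit actors implementing InteractInterface_Kostin.
; BeginPlay is empty, and the WBP_Main widget creation is disconnected, so it never runs.
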(event EventBeginPlay)

(event Collision|EventActorBeginOverlap
  (params (OtherActor :type Actor%20Object%20Reference)))

(event EventTick
  (params (DeltaSeconds :type Float%20%28single-precision%29)))

(event Input|KeyboardEvents|DebugKeyE
  (params (Key :type Key%20Structure :default "None") (ActionValue :type Input%20Action%20Value%20Structure))
  (bind _returnvalue (Transformation|GetActorLocation))
  (:Pressed
    (bind _outhit (Collision|SphereTraceByChannel _returnvalue (+ _returnvalue (* (Math|Vector|GetForwardVector (Variables|Default|GetCamera)) 3e+02)) 2e+01 "TraceTypeQuery1" false 0 "ForDuration"))
    (if (.bBlockingHit (Collision|BreakHitResult _outhit))
      (Utilities|IsValid (.HitActor (Collision|BreakHitResult _outhit))
        (:Is%20Valid
          (if (Utilities|DoesObjectImplementInterface (.HitActor (Collision|BreakHitResult _outhit)) "/Script/TMS_LS.InteractInterface_Kostin")
            (Class|InteractInterfaceKostin|InteractCall(Message) (.HitActor (Collision|BreakHitResult _outhit)) (Game|GetPlayerController 0))))))))

(event Input|KeyboardEvents|DebugKeyT
  (params (Key :type Key%20Structure :default "None") (ActionValue :type Input%20Action%20Value%20Structure))
  (:Pressed
    (bind _outitemdata (Class|GameInstanceSubsystemKostin|GetItemDatabyID (Subsystems|GetGameInstanceSubsystemKostin)))
    (Development|PrintString (Utilities|String|ToString(Text) (.Name (Utilities|Struct|BreakItemData_Kostin _outitemdata))))))

(fn ConstructionScript)